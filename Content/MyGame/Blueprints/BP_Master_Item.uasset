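; BP_Master_Item is an item Blueprint that makes itself available for pickup when the player is near.
; Overlapping InteractColission registers the item as BP_Player's ItemToPickup, shows the pickup notifier and switches the player's pending state.
; Leaving clears all three only if this item is still the registered one, so overlapping items do not cancel each other.
; The pickup itself is not handled here.
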(event OnComponentEndOverlap(InteractColission)
  (params (OverlappedComponent :type Primitive%20Component%20Object%20Reference) (OtherActor :type Actor%20Object%20Reference) (OtherComp :type Primitive%20Component%20Object%20Reference) (OtherBodyIndex :type Integer))
  (bind _asbp_player (Utilities|Casting|CastToBP_Player OtherActor))
  (if (== (Variables|/Game/MyGame/Blueprints/BP_Player.BP_Player_C|GetItemToPickup _asbp_player) self)
    (Variables|/Game/MyGame/Blueprints/BP_Player.BP_Player_C|SetItemToPickup _asbp_player 0)
    (Default|FShowPickupNotifier _asbp_player "Hidden")
    (Variables|/Game/MyGame/Blueprints/BP_Player.BP_Player_C|SetE_PendingState _asbp_player "NewEnumerator0")))

(event OnComponentBeginOverlap(InteractColission)
  (params (OverlappedComponent :type Primitive%20Component%20Object%20Reference) (OtherActor :type Actor%20Object%20Reference) (OtherComp :type Primitive%20Component%20Object%20Reference) (OtherBodyIndex :type Integer) (bFromSweep :type Boolean) (SweepResult :type Hit%20Result%20Structure%20%28by%20ref%29))
  (bind _asbp_player (Utilities|Casting|CastToBP_Player OtherActor))
  (Variables|/Game/MyGame/Blueprints/BP_Player.BP_Player_C|SetItemToPickup _asbp_player self)
  (Default|FShowPickupNotifier _asbp_player "Visible")
  (Variables|/Game/MyGame/Blueprints/BP_Player.BP_Player_C|SetE_PendingState _asbp_player "NewEnumerator1"))

(event EventBeginPlay)

(event Collision|EventActorBeginOverlap
  (params (OtherActor :type Actor%20Object%20Reference)))

(event EventTick
  (params (DeltaSeconds :type Float%20%28single-precision%29)))

(fn ConstructionScript)