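; BP_EnemyAI is an enemy character that roams randomly and chases players who come within its aggro range.
; Roaming walks slowly to random reachable points nearby, repeating after a short pause while it has no aggro.
; AggoSphere overlaps track players in range, targeting each new entrant for a faster, self-repeating AIMoveTo chase.
; Any player leaving clears aggro and restarts roaming, and both move loops repeat only on success.
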(event OnComponentBeginOverlap(AggoSphere)
  (params (OverlappedComponent :type Primitive%20Component%20Object%20Reference) (OtherActor :type Actor%20Object%20Reference) (OtherComp :type Primitive%20Component%20Object%20Reference) (OtherBodyIndex :type Integer) (bFromSweep :type Boolean) (SweepResult :type Hit%20Result%20Structure%20%28by%20ref%29))
  (bind _asbp_player (Utilities|Casting|CastToBP_Player OtherActor))
  (Utilities|Array|Add (Variables|Default|GetPlayerInRange) _asbp_player)
  (Variables|Default|SetHasAggo true)
  (bind _output_get (Variables|Default|SetTarget _asbp_player))
  (CallFunction|EventChasePlayer))

(event OnComponentEndOverlap(AggoSphere)
  (params (OverlappedComponent :type Primitive%20Component%20Object%20Reference) (OtherActor :type Actor%20Object%20Reference) (OtherComp :type Primitive%20Component%20Object%20Reference) (OtherBodyIndex :type Integer))
  (bind _asbp_player (Utilities|Casting|CastToBP_Player OtherActor))
  (Utilities|Array|RemoveItem (Variables|Default|GetPlayerInRange) _asbp_player)
  (Variables|Default|SetHasAggo false)
  (CallFunction|EventRoam))

(event Custom|Event_Roam
  (Variables|/Script/Engine.CharacterMovementComponent|SetMaxWalkSpeed (Variables|Character|GetCharacterMovement) 1e+02)
  (AI|AIMoveTo self (.RandomLocation (AI|Navigation|GetRandomReachablePointinRadius (Transformation|GetActorLocation) 1e+03 0 0)) 0 5.0 false
    (:OnSuccess
      (Utilities|FlowControl|Delay 1.0)
      (if (not (Variables|Default|GetHasAggo))
        (CallFunction|EventRoam)))))

(event Custom|Event_ChasePlayer
  (Variables|/Script/Engine.CharacterMovementComponent|SetMaxWalkSpeed (Variables|Character|GetCharacterMovement) 4e+02)
  (AI|AIMoveTo self "0, 0, 0" (Variables|Default|GetTarget) 5.0 false
    (:OnSuccess
      (CallFunction|EventChasePlayer))))

(event EventBeginPlay
  (CallFunction|EventRoam))

(fn ConstructionScript)